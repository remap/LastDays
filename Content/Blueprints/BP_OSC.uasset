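; BP_OSC is a Blueprint that receives OSC messages and forwards them as sequencer commands.
; On BeginPlay it binds to its OscReceiver, then splits each incoming address on slashes, taking the segments after the first as Group, SequenceName and Action.
; It stores these values and passes them to OSCEvent on its BP_OSC_Sequencer component.
; Message data and sender IP go unused, and each received address is printed.
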(event Custom|OSCRx
  (params (Address :type Name%20%28by%20ref%29) (Data :type Array%20of%20Osc%20Data%20Elem%20Struct%20Structures) (SenderIp :type String))
  (bind (_returnvalue _group _sequencename _action) (|getVars))
  (bind _output_get (Variables|Default|SetrawAddress (Utilities|String|ToString(Name) Address)))
  (bind _output_get_2 (Variables|Default|SetparsedAddress (Utilities|String|ParseIntoArray _output_get "/")))
  (|setVars (.Output (|parseArray _output_get_2 _output_get_2 _output_get_2)) (.Output2 (|parseArray _output_get_2 _output_get_2 _output_get_2)) (.Output3 (|parseArray _output_get_2 _output_get_2 _output_get_2)))
  (Default|OSCEvent _returnvalue _group _sequencename _action)
  (Development|PrintString (Utilities|String|ToString(Name) Address)))

(event EventBeginPlay
  (EventDispatchers|BindEventtoOnOscReceived (Variables|Default|GetOscReceiver) (delegate Custom|OSCRx))
  (Development|PrintString "Started"))

(fn ConstructionScript)