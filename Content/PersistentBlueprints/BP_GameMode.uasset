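; Game mode that gives each joining player a random campus-building name as the OrbName on their BP_PlayerState at PostLogin.
; It also stores plane transforms by name and can spawn a plane from a name-to-class map at its saved transform, logging an error for unknown names.
; RespawnMissingPlanes is empty; its missing-plane scan and the post-spawn naming and tagging logic are disconnected and never run.
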(event EventBeginPlay)

(event EventTick
  (params (DeltaSeconds :type Float%20%28single-precision%29)))

(event EventPostLogin
  (params (NewPlayer :type Player%20Controller%20Object%20Reference))
  (bind _asbp_player_state (Utilities|Casting|CastToBP_PlayerState (Variables|/Script/Engine.Controller|GetPlayerState NewPlayer)))
  (Variables|/Game/PersistentBlueprints/BP_PlayerState.BP_PlayerState_C|SetorbName _asbp_player_state (Utilities|Array|Get(acopy) (Utilities|Array|MakeArray (Utilities|Text|MakeLiteralText "Anderson") (Utilities|Text|MakeLiteralText "Ackerman") (Utilities|Text|MakeLiteralText "Boelter") (Utilities|Text|MakeLiteralText "Broad") (Utilities|Text|MakeLiteralText "Bunche") (Utilities|Text|MakeLiteralText "Engineering IV") (Utilities|Text|MakeLiteralText "Engineering V") (Utilities|Text|MakeLiteralText "Engineering VI") (Utilities|Text|MakeLiteralText "Kerckhoff") (Utilities|Text|MakeLiteralText "Schoenberg") (Utilities|Text|MakeLiteralText "WG Young")) (Math|Random|RandomIntegerinRange 0 10))))

(fn ConstructionScript)

(fn SavePlaneTransform
  (params (planeName :type String) (transform :type Transform))
  (Utilities|Map|Add (Variables|Default|GetplaneTransforms) planeName transform))

(fn RespawnMissingPlanes
  (params (controller :type BP%20Player%20Controller%20Object%20Reference)))

(fn SpawnPlanebyName
  (params (planeName :type String) (owner :type BP%20Player%20Controller%20Object%20Reference))
  (bind _pawnclasses_ (Variables|Default|GetpawnClasses_))
  (bind (_value _returnvalue) (Utilities|Map|Find _pawnclasses_ planeName))
  (if _returnvalue
    (Game|SpawnActorfromClass _value (.Value (Utilities|Map|Find (Variables|Default|GetplaneTransforms) planeName)) "Undefined" owner 0)
    (else
      (Class|DDBlueprintLibrary|LogError (Utilities|String|ToString(Text) (Utilities|Text|FormatText "Fatal Error: Pawn class not found for {p}" (Utilities|Text|ToText(String) planeName)))))))