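; Blueprint function library that gives other Blueprints typed access to the project's game mode, player controller and game instance.
; Each getter fetches the engine object and casts it to BP_GameMode, BP_PlayerController or BP_MPGameInstance, logging an error if the cast fails.
; The player controller getter always uses player index 0.
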(fn GetMyGameMode
  (bind _asbp_game_mode (Utilities|Casting|CastToBP_GameMode (Game|GetGameMode))
    (:then
      (return _asbp_game_mode))
    (:CastFailed
      (Class|DDBlueprintLibrary|LogError "Get My Game Mode: Can't cast to BP_GameMode"))))

(fn GetMyPlayerController
  (bind _asbp_player_controller (Utilities|Casting|CastToBP_PlayerController (Game|GetPlayerController 0))
    (:then
      (return _asbp_player_controller))
    (:CastFailed
      (Class|DDBlueprintLibrary|LogError "Get My Player Controller: Can't cast to BP Player Controller"))))

(fn GetMyGameInstance
  (bind _asbp_mpgame_instance (Utilities|Casting|CastToBP_MPGameInstance (Game|GetGameInstance))
    (:then
      (return _asbp_mpgame_instance))
    (:CastFailed
      (Class|DDBlueprintLibrary|LogError "Get My Game Instance: Can't cast to BP_MPGameInstance"))))