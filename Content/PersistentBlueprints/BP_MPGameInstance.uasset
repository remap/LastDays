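; Multiplayer game instance that handles hosting, joining and disconnecting, and owns the persistent save game.
; Connections use "open" console commands on the Landscape level or a given IP, while the LAN session create, find and join nodes are left unwired.
; Init loads or creates BP_SaveGame, which helper functions use to store the pawn name and per-plane UV selection bounds.
; It also logs network failures and unpossesses the first player controller on shutdown.
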(event Custom|GameInstance_HostLobby
  (params (Host :type BP%20Player%20Controller%20Object%20Reference))
  (Development|ExecuteConsoleCommand "open Landscape?Listen" 0))

(event Custom|GameInstance_JoinLobby
  (params (Joining :type BP%20Player%20Controller%20Object%20Reference) (IP :type String))
  (Development|ExecuteConsoleCommand (Utilities|String|Append (Utilities|String|ToString(Text) (Utilities|Text|FormatText "open ")) IP) 0))

(event Custom|GameInstance_Disconnect
  (Development|ExecuteConsoleCommand "open Landscape" 0))

(event EventInit
  ;[1 0.8092 0] Comment
  (bind _returnvalue (SaveGame|LoadGamefromSlot (Variables|Default|GetsaveGameSlot)))
  (if (Utilities|IsValid _returnvalue)
    (bind _asbp_save_game (Utilities|Casting|CastToBP_SaveGame _returnvalue)
      (:then
        (Variables|Default|SetsaveGame _asbp_save_game))
      (:CastFailed
        (bind _returnvalue_2 (SaveGame|CreateSaveGameObject "/Game/PersistentBlueprints/BP_SaveGame.BP_SaveGame_C" :!label _label))
        (SaveGame|SaveGametoSlot _returnvalue_2 (Variables|Default|GetsaveGameSlot))
        (Variables|Default|SetsaveGame _returnvalue_2)))
    (else
      (goto _label))))

(event EventHandleNetworkError
  (params (FailureType :type ENetworkFailure%20Enum :default "NetDriverAlreadyExists") (bIsServer :type Boolean))
  (switch Utilities|FlowControl|Switch|SwitchonENetworkFailure FailureType
    (:NetDriverAlreadyExists
      (Class|DDBlueprintLibrary|LogError "Network Error: Net driver already exists"))
    (:NetDriverCreateFailure
      (Class|DDBlueprintLibrary|LogError "Network Error: Net driver create failure"))
    (:NetDriverListenFailure
      (Class|DDBlueprintLibrary|LogError "Network Error: Net driver listen failure"))
    (:ConnectionLost
      (Class|DDBlueprintLibrary|LogError "Network Error: Connectionn lost"))
    (:ConnectionTimeout
      (Class|DDBlueprintLibrary|LogError "Network Error: Connectionn timeout"))
    (:FailureReceived
      (Class|DDBlueprintLibrary|LogError "Network Error: Failure Received"))
    (:OutdatedClient
      (Class|DDBlueprintLibrary|LogError "Network Error: Outdated client"))
    (:OutdatedServer
      (Class|DDBlueprintLibrary|LogError "Network Error: Outdated server"))
    (:PendingConnectionFailure
      (Class|DDBlueprintLibrary|LogError "Network Error: Pending connection failure"))
    (:NetGuidMismatch
      (Class|DDBlueprintLibrary|LogError "Network Error: Net guid mismatch"))
    (:NetChecksumMismatch
      (Class|DDBlueprintLibrary|LogError "Network Error: Net checksum mismatch"))))

(event EventShutdown
  (Class|DDBlueprintLibrary|LogWarning "Game ShutDown Started...")
  (Pawn|UnPossess (Game|GetPlayerController 0)))

(fn GetUVMappingforPlane
  (params (planeName :type String))
  (bind _savegame (Variables|Default|GetsaveGame))
  (bind _planeselectionstart (Variables|/Game/PersistentBlueprints/BP_SaveGame.BP_SaveGame_C|GetplaneSelectionStart _savegame))
  (bind _planeselectionend (Variables|/Game/PersistentBlueprints/BP_SaveGame.BP_SaveGame_C|GetplaneSelectionEnd _savegame))
  (bind (_value _returnvalue) (Utilities|Map|Find _planeselectionstart planeName))
  (bind (_value_2 _returnvalue_2) (Utilities|Map|Find _planeselectionend planeName))
  (if _returnvalue
    (if _returnvalue_2
      (return _value _value_2)
      (else
        _)))
  (return "" "(X=1.000000,Y=1.000000)"))

(fn SetUVMappingforPlane
  (params (planeName :type String) (planeSelectStart :type Vector%202D%20Structure) (planeSelectEnd :type Vector%202D%20Structure))
  (bind _savegame (Variables|Default|GetsaveGame))
  (Utilities|Map|Add (Variables|/Game/PersistentBlueprints/BP_SaveGame.BP_SaveGame_C|GetplaneSelectionStart _savegame) planeName planeSelectStart)
  (Utilities|Map|Add (Variables|/Game/PersistentBlueprints/BP_SaveGame.BP_SaveGame_C|GetplaneSelectionEnd _savegame) planeName planeSelectEnd)
  (SaveGame|SaveGametoSlot _savegame (Variables|Default|GetsaveGameSlot)))

(fn ShowUVMappings
  (bind _savegame (Variables|Default|GetsaveGame))
  (bind _planeselectionstart (Variables|/Game/PersistentBlueprints/BP_SaveGame.BP_SaveGame_C|GetplaneSelectionStart _savegame))
  (bind _keys (Utilities|Map|Keys _planeselectionstart))
  (for _array_element _keys
    (Class|DDBlueprintLibrary|LogDebug (Utilities|String|ToString(Text) (Utilities|Text|FormatText "Mapping  {n}: {uv1} {uv2}" (Utilities|Text|ToText(String) _array_element) (Utilities|Text|ToText(String) (.Value (Utilities|Map|Find _planeselectionstart _array_element))) (Utilities|Text|ToText(String) (.Value (Utilities|Map|Find (Variables|/Game/PersistentBlueprints/BP_SaveGame.BP_SaveGame_C|GetplaneSelectionEnd _savegame) _array_element))))))))

(fn LoadPawnName
  (return (Variables|/Game/PersistentBlueprints/BP_SaveGame.BP_SaveGame_C|GetmyPawnName (Variables|Default|GetsaveGame))))

(fn SavePawnName
  (params (name :type String))
  (bind _savegame (Variables|Default|GetsaveGame))
  (Variables|/Game/PersistentBlueprints/BP_SaveGame.BP_SaveGame_C|SetmyPawnName _savegame name)
  (SaveGame|SaveGametoSlot _savegame (Variables|Default|GetsaveGameSlot)))