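; BP_ShellAppLibrary is a function library of shared lookup helpers for players, pawns and auto-follow targets.
; It returns the first player's BP_PlayerController, a list of player controllers built from the game mode's player count, and all pawns in the world, optionally excluding the local controlled pawn.
; The auto-follow list is currently just every pawn, including the player's own.
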(fn GetMyController
  (bind _asbp_player_controller (Utilities|Casting|CastToBP_PlayerController (Game|GetPlayerController 0)))
  (return _asbp_player_controller))

(fn GetAllPlayers
  (bind _returnvalue (Class|GameModeBase|GetNumPlayers (Game|GetGameMode)))
  (for _index (range 0 (- _returnvalue 1))
    (Utilities|Array|Add (LocalVariables|Getplayers) (Game|GetPlayerController 0 _index)))
  (return (LocalVariables|Getplayers)))

(fn GetAllPawns
  (params (excludeMine :type Boolean))
  (bind _outactors (Actor|GetAllActorsOfClass 0 "/Script/Engine.Pawn"))
  (bind _output_get (LocalVariables|Setactors _outactors))
  (if excludeMine
    (Utilities|Array|RemoveItem _output_get (Pawn|GetControlledPawn (CallFunction|GetMyController))))
  (return (LocalVariables|Getactors)))

(fn GetAllAutoFollowActors
  (Utilities|Array|AppendArray (LocalVariables|GetafActors) (CallFunction|GetAllPawns false))
  (return (LocalVariables|GetafActors)))