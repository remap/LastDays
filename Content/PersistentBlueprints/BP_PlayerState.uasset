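; Player state that tracks progress through the shore, rocks, museum and invention pods and sets where the guide orb goes next.
; UpdatePlayerState records a pod's state, runs a decision tree that alternates later museum and invention parts, picks a hard-coded location, then fires ForwardStateUpdateToSublevel.
; Guiding can be disabled, clearing OrbActive.
; It also applies the replicated orb name to the orb pawn and relays tagged sequence playback to the local player controller.
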(event Custom|UpdatePlayerState
  (params (Active :type Boolean) (Pod :type String) (State :type Integer))
  (if (Variables|Default|GetGuidingDisabled)
    (Variables|Default|SetOrbActive false)
    (else
      (Variables|Default|SetOrbActive Active)))
  (Utilities|Map|Add (Variables|Default|GetPodStates) Pod State)
  (CallFunction|UpdateGuideGoal)
  (Default|CallForwardStateUpdatetoSublevel)
  (Development|PrintString (Variables|Default|GetGuideCurrentPod) true true "(R=0.000000,G=0.660000,B=1.000000,A=1.000000)" 8.0))

(event Custom|SetGuidingDisabled
  (params (DisableGuiding :type Boolean))
  (bind _output_get (Variables|Default|SetGuidingDisabled DisableGuiding))
  (CallFunction|UpdatePlayerState (not _output_get) "none"))

(event Custom|RPC%20Mcast%20Set%20Tagged%20Sequence%20Playback
  (params (tag :type Name) (play :type Boolean) (seek%20pos :type Float%20%28single-precision%29) (seek :type Boolean) (seel%20relative :type Boolean) (toggle :type Boolean) (grouptag :type Name))
  (bind _asbp_player_controller (Utilities|Casting|CastToBP_PlayerController (Game|GetPlayerController 0)))
  (Default|SetTaggedSequencePlayback _asbp_player_controller tag play seek%20pos seek seel%20relative toggle grouptag))

(event EventBeginPlay)

(event EventTick
  (params (DeltaSeconds :type Float%20%28single-precision%29)))

(fn ConstructionScript)

(fn OnRepPlayerOrbPawn)

(fn OnRepOrbName
  (bind _orbname (Variables|Default|GetorbName))
  (bind _playerorbpawn (Variables|Default|GetplayerOrbPawn))
  (bind _asbp_orb_pawn (Utilities|Casting|CastToBP_OrbPawn (Variables|Default|GetPawnPrivate))
    (:then
      (Default|SetOrbName _asbp_orb_pawn _orbname))
    (:CastFailed
      (Utilities|IsValid _playerorbpawn
        (:Is%20Valid
          (Default|SetOrbName _playerorbpawn _orbname))))))

(fn UpdateGuideGoal
  (bind _podstates (Variables|Default|GetPodStates))
  (LocalVariables|Setshore (.Value (Utilities|Map|Find _podstates "shore")))
  (LocalVariables|Setrocks (.Value (Utilities|Map|Find _podstates "rocks")))
  (LocalVariables|Setmuseum (.Value (Utilities|Map|Find _podstates "museum")))
  (LocalVariables|Setinvention (.Value (Utilities|Map|Find _podstates "invention")))
  (if (Math|Boolean|ANDBoolean (< (LocalVariables|Getshore) 3) (== 0 (LocalVariables|Getrocks)) (and (== 0 (LocalVariables|Getmuseum)) (== 0 (LocalVariables|Getinvention))))
    ;[1 1 1] Still on shore
    (Variables|Default|SetGuideCurrentPod "shore")
    (CallFunction|ShoreLocations)
    (elif (and (== 0 (LocalVariables|Getmuseum)) (== 0 (LocalVariables|Getinvention)))
      (if (<= (LocalVariables|Getrocks) 4)
        ;[1 1 1] Rocks incomplete
        (Variables|Default|SetGuideCurrentPod "rocks")
        (CallFunction|RocksLocations)
        (else
          ;[1 1 1] Rocks finished and museum not started yet
          (Variables|Default|SetGuideCurrentPod "museum")
          (CallFunction|MuseumLocations)))
      (elif (< (LocalVariables|Getmuseum) 4)
        ;[1 1 1] Museum Part 1
        (Variables|Default|SetGuideCurrentPod "museum")
        (CallFunction|MuseumLocations)
        (elif (< (LocalVariables|Getinvention) 2)
          ;[1 1 1] Go to Invention Part 1
          (Variables|Default|SetGuideCurrentPod "invention")
          (CallFunction|InventionLocations)
          (elif (< (LocalVariables|Getmuseum) 6)
            ;[1 1 1] Museum Part 2
            (Variables|Default|SetGuideCurrentPod "museum")
            (CallFunction|MuseumLocations)
            (else
              ;[1 1 1] Go to Invention Part 2
              (Variables|Default|SetGuideCurrentPod "invention")
              (CallFunction|InventionLocations))))))))

(fn ShoreLocations
  (switch int (.Value (Utilities|Map|Find (Variables|Default|GetPodStates) "shore"))
    (:0
      (Variables|Default|SetNextOrbLoc "13713.000000,1570.000000,800.000000"))
    (:1
      (Variables|Default|SetNextOrbLoc "10170.000000,5080.000000,1190.000000"))
    (:2
      (Variables|Default|SetNextOrbLoc "7500.000000,10000.000000,900.000000"))
    (:3
      (Variables|Default|SetNextOrbLoc "2500.000000,9000.000000,3000.000000"))))

(fn RocksLocations
  (switch int (.Value (Utilities|Map|Find (Variables|Default|GetPodStates) "rocks"))
    (:0
      (Variables|Default|SetNextOrbLoc "-232.000000,6034.071289,4050.039063"))
    (:1
      (Variables|Default|SetNextOrbLoc "-5032.000000,-7985.000000,4660.000000"))
    (:2
      (Variables|Default|SetNextOrbLoc "-800.000000,-15811.000000,500.000000"))
    (:3
      (Variables|Default|SetNextOrbLoc "-1450.000000,-11500.000000,1500.000000"))
    (:4
      (Variables|Default|SetNextOrbLoc "-5732.000000,-10100.000000,3360.000000"))))

(fn MuseumLocations
  (switch int (.Value (Utilities|Map|Find (Variables|Default|GetPodStates) "museum"))
    (:0
      (Variables|Default|SetNextOrbLoc "-5000.000000,-3000.000000,4600.000000"))
    (:1
      (Variables|Default|SetNextOrbLoc "4000.000000,-2500.000000,4600.000000"))
    (:2
      (Variables|Default|SetNextOrbLoc "740.000000,-5900.000000,4600.000000" :!label _label))
    (:3
      (Variables|Default|SetNextOrbLoc "4700.000000,-6000.000000,4600.000000" :!label _label_2))
    (:4
      (goto _label))
    (:5
      (goto _label_2))))

(fn InventionLocations
  (switch int (.Value (Utilities|Map|Find (Variables|Default|GetPodStates) "invention"))
    (:0
      (Variables|Default|SetNextOrbLoc "-400.000000,-7450.000000,4650.000000" :!label _label))
    (:1
      (Variables|Default|SetNextOrbLoc "4900.000000,-6400.000000,4650.000000"))
    (:2
      (goto _label))))