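; BP_OrbPawn is a networked player orb pawn with a randomly colored emissive material and a name label.
; Non-server instances send their transform each tick through an RPC into PawnTransform, whose RepNotify applies it.
; After a short delay, BeginPlay reads the orb name from BP_PlayerState for the label and actor tag.
; The V key toggles first- and third-person cameras, switching controller-rotation following to match.
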(event Custom|RPC_ReplicateTransform
  (params (transform :type Transform))
  (Variables|Default|SetpawnTransform transform))

(event EventBeginPlay
  (bind _returnvalue (Math|Random|RandomFloatinRange 0.0 0.6))
  (bind _returnvalue_2 (Math|Random|RandomFloatinRange 0.1 0.8))
  (bind _returnvalue_3 (Math|Random|RandomFloatinRange 0.0 3.6e+02))
  (bind _returnvalue_4 (Class|KismetMathLibrary|HSVtoRGB _returnvalue_3 _returnvalue_2 _returnvalue 1.0))
  (bind _returnvalue_5 (Rendering|Material|CreateDynamicMaterialInstance (Variables|GetMeshComponent) 0 "/Game/Materials/M_BaseEmissiveMat.M_BaseEmissiveMat" "None" :!class /Script/Engine.PrimitiveComponent))
  (Rendering|Material|SetVectorParameterValue _returnvalue_5 "Color" _returnvalue_4 :!class /Script/Engine.MaterialInstanceDynamic)
  (Variables|Default|SetPlayerColor _returnvalue_4)
  (Input|EnableInput (Game|GetPlayerController 0))
  (Utilities|FlowControl|Delay 1.0)
  (bind _asbp_player_state (Utilities|Casting|CastToBP_PlayerState (Variables|GetPlayerState)))
  (CallFunction|SetOrbName (Variables|/Game/PersistentBlueprints/BP_PlayerState.BP_PlayerState_C|GetorbName _asbp_player_state)))

(event EventTick
  (params (DeltaSeconds :type Float%20%28single-precision%29))
  (if (not (Networking|IsServer))
    (CallFunction|RPCReplicateTransform (Transformation|GetActorTransform))))

(event Input|KeyboardEvents|V
  (params (Key :type Key%20Structure :default "None"))
  (bind _fp_camera (Variables|Default|GetFP_Camera))
  ;[1 1 1] 1st/3rd person camera switch
  (:Pressed
    (Utilities|FlowControl|MultiGate false true -1
      (:Out%200
        (Variables|/Script/Engine.SpringArmComponent|SetTargetArmLength (Variables|Default|GetSpringArm) 3e+02)
        (Components|Activation|SetActive (Variables|Default|GetFP_Camera) false false)
        (Components|Activation|SetActive (Variables|Default|GetTP_Camera) true false)
        (Variables|Default|SetbUseControllerRotationPitch false)
        (Variables|Default|SetbUseControllerRotationRoll false)
        (Variables|Default|SetbUseControllerRotationYaw false))
      (:Out%201
        (Components|Activation|SetActive _fp_camera true false)
        (Components|Activation|SetActive (Variables|Default|GetTP_Camera) false true)
        (Transformation|SetRelativeLocation _fp_camera "0, 0, 0" false false)
        (Variables|Default|SetbUseControllerRotationPitch true)
        (Variables|Default|SetbUseControllerRotationRoll true)
        (Variables|Default|SetbUseControllerRotationYaw true)))))

(fn ConstructionScript)

(fn OnRepPlayerColor)

(fn OnRepPawnTransform
  (Transformation|SetActorTransform (Variables|Default|GetpawnTransform)))

(fn UpdateTags
  (params (newName :type Text))
  (Variables|Default|SetTags (Utilities|Array|MakeArray (Utilities|String|StringToName (Utilities|String|ToString(Text) newName)))))

(fn SetOrbName
  (params (newName :type Text))
  (Rendering|Components|TextRender|SetText (Variables|Default|GetOrbNameRender) newName)
  (CallFunction|UpdateTags newName))